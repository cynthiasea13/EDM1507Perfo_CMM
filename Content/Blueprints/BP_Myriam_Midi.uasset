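; BP_Myriam_Midi is a Blueprint that receives MIDI input from a chosen hardware device and prints it on screen for debugging.
; On BeginPlay it scans the MIDI devices, creates a controller for the input device matching MIDIControllerIndex, and binds its MIDI event.
; Each event stores its type, control ID and velocity, prints them, then reaches a switch on event type with no actions attached.
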(event `self.ReceiveBeginPlay`
  (bind _outmididevices (`MIDIDeviceManager.FindMIDIDevices`))
  (for _array_element _outmididevices
    (bind (_deviceid _devicename _bcanreceivefrom) (break `FoundMIDIDevice` _array_element))
    (if _bcanreceivefrom
      (if (== (`self.MIDIControllerIndex`) _deviceid)
        (`KismetSystemLibrary.PrintString` (`KismetTextLibrary.Conv_TextToString` (`|FormatText` "{ID} {Nom} " _deviceid _devicename)) true true (struct :`G` 0.66 :`B` 1.0 :`A` 1.0) 30.0)
        (bind _returnvalue (`MIDIDeviceManager.CreateMIDIDeviceController` _deviceid))
        (bind _output_get (set `self.MIDIControl` _returnvalue))
        (add `MIDIDeviceController.OnMIDIEvent` _output_get (`|CreateDelegate` :!event `OnMidiEvent`)))))
  (`KismetSystemLibrary.PrintString` "BOUCLE TERMINÉE" true true (struct :`R` 0.425 :`B` 0.041941 :`A` 1.0) 30.0))

(event `OnMidiEvent`
  (params (MIDIDeviceController :type "MIDIDeviceController Object Reference") (Timestamp :type Integer) (EventType :type "EMIDIEventType Enum" :default "Unknown") (Channel :type Integer) (ControlID :type Integer) (Velocity :type Integer) (RawEventType :type Integer))
  (set `self.Event Type` EventType)
  (set `self.Control ID` ControlID)
  (set `self.Velocity` Velocity)
  (`KismetSystemLibrary.PrintString` (`KismetTextLibrary.Conv_TextToString` (`|FormatText` "MIDI EVENT TYPE {event} MIDI Note {note} VELOCITE {velocite}" (`|GetEnumeratorNameAsString` EventType) ControlID Velocity)) true true (struct :`R` 0.425 :`B` 0.041941 :`A` 1.0) 2.0 "MIDI2")
  (switch `EMIDIEventType` (`self.Event Type`)))

(fn `UserConstructionScript`)