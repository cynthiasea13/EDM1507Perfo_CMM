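; Actor that runs a kick, snare and hi-hat drum machine controlled live from a MIDI controller.
; On BeginPlay it opens the MIDI input matching MIDIControllerIndex, then creates three 2D sounds, passes them the MainClock BPM and starts them bar-quantized on that Quartz clock.
; Incoming Control Change messages are normalized to 0–1 and drive each sound's volume and one timbre parameter.
; Devices and MIDI events are printed on screen for debugging.
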(event `self.ReceiveBeginPlay`
  (bind _outmididevices (`MIDIDeviceManager.FindMIDIDevices`))
  (for _array_element _outmididevices
    (bind (_deviceid _devicename _bcanreceivefrom) (break `FoundMIDIDevice` _array_element))
    (if _bcanreceivefrom
      (if (== (`self.MIDIControllerIndex`) _deviceid)
        (`KismetSystemLibrary.PrintString` (`KismetTextLibrary.Conv_TextToString` (`|FormatText` "{ID} {Nom} " _deviceid _devicename)) true true (struct :`G` 0.66 :`B` 1.0 :`A` 1.0) 30.0)
        (bind _returnvalue (`MIDIDeviceManager.CreateMIDIDeviceController` _deviceid))
        (bind _output_get (set `self.MIDIControl` _returnvalue))
        (add `MIDIDeviceController.OnMIDIEvent` _output_get (`|CreateDelegate` :!event `OnMidiEvent`)))))
  (`KismetSystemLibrary.PrintString` "BOUCLE TERMINÉE" true true (struct :`R` 0.276797 :`G` 0.203429 :`B` 1.0 :`A` 1.0) 30.0)
  (bind _returnvalue_2 (`GameplayStatics.CreateSound2D` "/Game/Metasound/Marianne/MSSkick.MSSkick" 1.0 1.0 0.0 null))
  (bind _output_get_2 (set `self.BPsequ` _returnvalue_2))
  (`AudioParameterControllerInterface.SetFloatParameter` _output_get_2 "BPM" (`/Game/Blueprints/BP_EDM1507_Clock.Beats Per Minute` (`self.MainClock`)))
  (`AudioComponent.PlayQuantized` :`self` _output_get_2 :`InClockHandle` (`/Game/Blueprints/BP_EDM1507_Clock.MainClock` (`self.MainClock`)) :`InQuantizationBoundary` (make `QuartzQuantizationBoundary` "Bar" 1.0 "CurrentTimeRelative"))
  (bind _returnvalue_3 (`GameplayStatics.CreateSound2D` "/Game/Metasound/Marianne/MSSHihat.MSSHihat" 1.0 1.0 0.0 null))
  (bind _output_get_3 (set `self.Hihat` _returnvalue_3))
  (`AudioParameterControllerInterface.SetFloatParameter` _output_get_3 "BPM" (`/Game/Blueprints/BP_EDM1507_Clock.Beats Per Minute` (`self.MainClock`)))
  (`AudioComponent.PlayQuantized` :`self` _output_get_3 :`InClockHandle` (`/Game/Blueprints/BP_EDM1507_Clock.MainClock` (`self.MainClock`)) :`InQuantizationBoundary` (make `QuartzQuantizationBoundary` "Bar" 1.0 "CurrentTimeRelative"))
  (bind _returnvalue_4 (`GameplayStatics.CreateSound2D` "/Game/Metasound/Marianne/MSSsnare.MSSsnare" 1.0 1.0 0.0 null))
  (bind _output_get_4 (set `self.snare` _returnvalue_4))
  (`AudioParameterControllerInterface.SetFloatParameter` _output_get_4 "BPM" (`/Game/Blueprints/BP_EDM1507_Clock.Beats Per Minute` (`self.MainClock`)))
  (`AudioComponent.PlayQuantized` :`self` _output_get_4 :`InClockHandle` (`/Game/Blueprints/BP_EDM1507_Clock.MainClock` (`self.MainClock`)) :`InQuantizationBoundary` (make `QuartzQuantizationBoundary` "Bar" 1.0 "CurrentTimeRelative")))

(event `OnMidiEvent`
  (params (MIDIDeviceController :type "MIDIDeviceController Object Reference") (Timestamp :type Integer) (EventType :type "EMIDIEventType Enum" :default "Unknown") (Channel :type Integer) (ControlID :type Integer) (Velocity :type Integer) (RawEventType :type Integer))
  (set `self.Event Type` EventType)
  (set `self.Control ID` ControlID)
  (set `self.Velocity` Velocity)
  (`KismetSystemLibrary.PrintString` (`KismetTextLibrary.Conv_TextToString` (`|FormatText` "MIDI EVENT TYPE {event} MIDI Note {note} VELOCITE {velocite}" (`|GetEnumeratorNameAsString` EventType) ControlID Velocity)) true true (struct :`R` 0.276797 :`G` 0.203429 :`B` 1.0 :`A` 1.0) 2.0 "MIDI1")
  (switch `EMIDIEventType` (`self.Event Type`)
    (:`ControlChange`
      (switch `string` (`KismetStringLibrary.Conv_IntToString` (`self.Control ID`))
        (:`70`
          (`AudioParameterControllerInterface.SetFloatParameter` (`self.BPsequ`) "Vol" (/ (`KismetMathLibrary.Conv_IntToDouble` (`self.Velocity`)) 127.0)))
        (:`71`
          (`AudioParameterControllerInterface.SetFloatParameter` (`self.snare`) "SnVol" (/ (`KismetMathLibrary.Conv_IntToDouble` (`self.Velocity`)) 127.0)))
        (:`72`
          (`AudioParameterControllerInterface.SetFloatParameter` (`self.Hihat`) "HHVol" (/ (`KismetMathLibrary.Conv_IntToDouble` (`self.Velocity`)) 127.0)))
        (:`74`
          (`AudioParameterControllerInterface.SetFloatParameter` (`self.BPsequ`) "BDFreq" (/ (`KismetMathLibrary.Conv_IntToDouble` (`self.Velocity`)) 127.0)))
        (:`75`
          (`AudioParameterControllerInterface.SetFloatParameter` (`self.snare`) "NoiseSN" (/ (`KismetMathLibrary.Conv_IntToDouble` (`self.Velocity`)) 127.0)))
        (:`76`
          (`AudioParameterControllerInterface.SetFloatParameter` (`self.Hihat`) "DKHH" (/ (`KismetMathLibrary.Conv_IntToDouble` (`self.Velocity`)) 127.0)))))))

(fn `UserConstructionScript`)